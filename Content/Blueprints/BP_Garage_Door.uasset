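; Garage door actor that opens when a component tagged "hand" overlaps its static mesh trigger.
; A DoOnce lets the first such overlap play a 2D sound and start a timeline; nothing resets it, so the door never closes.
; The timeline lerps the Door's relative location upward along Z from the position cached at BeginPlay.
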(event OnComponentBeginOverlap(StaticMeshComponent)
  (params (OverlappedComponent :type Primitive%20Component%20Object%20Reference) (OtherActor :type Actor%20Object%20Reference) (OtherComp :type Primitive%20Component%20Object%20Reference) (OtherBodyIndex :type Integer) (bFromSweep :type Boolean) (SweepResult :type Hit%20Result%20Structure%20%28by%20ref%29))
  (bind _startlocation (Variables|Default|GetStartLocation))
  (if (Components|ComponentHasTag OtherComp "hand")
    (Utilities|FlowControl|DoOnce false
      (:Completed
        (Audio|PlaySound2D "/Game/Sounds/garage_door.garage_door" 1.0 1.0 0.0 0 0)
        (bind _up (Timeline|Timeline Play)
          (:Update
            (Transformation|SetRelativeLocation (Variables|Default|Getdoor) (Math|Vector|Lerp(Vector) _startlocation (+ _startlocation "0.000000,0.000000,380.000000") _up) false false)))))))

(event EventBeginPlay
  (Variables|Default|SetStartLocation (Variables|/Script/Engine.SceneComponent|GetRelativeLocation (Variables|Default|Getdoor))))

(event Collision|EventActorBeginOverlap
  (params (OtherActor :type Actor%20Object%20Reference)))

(event EventTick
  (params (DeltaSeconds :type Float%20%28single-precision%29)))

(fn ConstructionScript)