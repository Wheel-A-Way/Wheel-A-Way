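; BP_GameEnd is the end-of-game sequence actor, holding a hidden widget and a car.
; Its showEndGame event reveals the widget, plays a thanks sound, waits, then plays a car-stop sound and starts the BringCar timeline.
; The timeline update sets the car between its stored start and an X offset, but the lerp alpha is fixed at zero.
; QuitGame follows in that same update, so the game quits on the first tick.
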(event Custom|showEndGame
  (bind _startlocation (Variables|Default|GetStartLocation))
  (Rendering|SetVisibility (Variables|Default|GetWidget) true false)
  (Audio|PlaySound2D "/Game/Sounds/Voicelines/M-_thanks.M-_thanks" 1.0 1.0 0.0 0 0)
  (Utilities|FlowControl|Delay 7.0)
  (Audio|PlaySound2D "/Game/Sounds/car_stop.car_stop" 1.0 1.0 0.0 0 0)
  (Timeline|bringCar Play
    (:Update
      (Transformation|SetRelativeLocation (Variables|Default|Getcar) (Math|Vector|Lerp(Vector) _startlocation (+ _startlocation "500.000000,0.000000,0.000000") 0.0) false false)
      (Game|QuitGame 0 "Quit" false))))

(event EventBeginPlay
  (Rendering|SetVisibility (Variables|Default|GetWidget) false false)
  (Variables|Default|SetStartLocation (Variables|/Script/Engine.SceneComponent|GetRelativeLocation (Variables|Default|Getcar))))

(fn ConstructionScript)