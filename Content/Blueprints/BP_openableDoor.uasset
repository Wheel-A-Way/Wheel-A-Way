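; BP_openableDoor is a door that swings open or shut when a component tagged "hand" begins overlapping its mesh.
; The overlap plays a timeline from the start, using the Open or Close track, chosen by IsClosed, to set the mesh's relative yaw across a 90-degree swing.
; When the timeline finishes, IsClosed flips for the next touch; the toggleDoor event is empty.
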(event OnComponentBeginOverlap(StaticMeshComponent)
  (params (OverlappedComponent :type Primitive%20Component%20Object%20Reference) (OtherActor :type Actor%20Object%20Reference) (OtherComp :type Primitive%20Component%20Object%20Reference) (OtherBodyIndex :type Integer) (bFromSweep :type Boolean) (SweepResult :type Hit%20Result%20Structure%20%28by%20ref%29))
  (if (Components|ComponentHasTag OtherComp "hand")
    (bind (_direction _open _close) (Timeline|Timeline PlayFromStart)
      (:Update
        (if (Variables|Default|GetisClosed)
          (Transformation|SetRelativeRotation (Variables|Debug|GetStaticMeshComponent) (Math|Rotator|MakeRotator 0.0 0.0 (* _open -9e+01)) false false)
          (else
            (Transformation|SetRelativeRotation (Variables|Debug|GetStaticMeshComponent) (Math|Rotator|MakeRotator 0.0 0.0 (* _close -9e+01)) false false))))
      (:Finished
        (if (Variables|Default|GetisClosed)
          (Variables|Default|SetisClosed false)
          (else
            (Variables|Default|SetisClosed true)))))))

(event Custom|toggleDoor)

(fn ConstructionScript)